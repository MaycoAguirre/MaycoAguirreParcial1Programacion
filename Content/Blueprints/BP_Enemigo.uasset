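; BP_Enemigo is an enemy actor that moves by a velocity vector and can spawn BP_Proyectil projectiles.
; Tick adds Velocidad as a local offset each frame, without sweep or delta-time scaling.
; SpawnProyectil spawns a projectile at the enemy's location and passes it that same Velocidad.
; Setter functions assign Velocidad directly or as the VelocidadProyectil vector scaled by a factor; nothing in this Blueprint calls them or the spawn.
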(event `self.ReceiveBeginPlay`)

(event `self.ReceiveTick`
  (params (DeltaSeconds :type "Float (single-precision)"))
  (`self.K2_AddActorLocalOffset` (`self.Velocidad`)))

(fn `SpawnProyectil`
  (`|SpawnActorFromClass` "/Game/Blueprints/BP_Proyectil.BP_Proyectil_C" (`KismetMathLibrary.MakeTransform` (`self.K2_GetActorLocation`)) "Undefined" "MultiplyWithRoot" null (`self.Velocidad`) null))

(fn `UserConstructionScript`)

(fn `VelocidadEnemigo`
  (params (Velocidad :type "Vector Structure"))
  (set `self.Velocidad` Velocidad))

(fn `velocidadProyectil`
  (params (Velocidad :type "Float (double-precision)") (VelocidadProyectil :type "Vector Structure"))
  (bind _output_get (set `self.VelocidadProyectil2` Velocidad))
  (set `self.Velocidad` (`KismetMathLibrary.MakeVector` (* _output_get VelocidadProyectil_X) (* _output_get VelocidadProyectil_Y) (* _output_get VelocidadProyectil_Z))))